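; Mutant Druid enemy character with melee attacks, health and death.
; Attack stops movement and plays one of two random montages, gated by a DoOnce until AttackEnded restores speed.
; Hand capsules, toggled by collision enable/disable events, deal random damage to other actors they overlap.
; Tick updates a health bar facing the player's camera; lethal damage triggers the death animation, disables capsule collision and destroys the actor after a delay.
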(event OnComponentBeginOverlap(CapsuleRigjtHand)
  (params (OverlappedComponent :type Primitive%20Component%20Object%20Reference) (OtherActor :type Actor%20Object%20Reference) (OtherComp :type Primitive%20Component%20Object%20Reference) (OtherBodyIndex :type Integer) (bFromSweep :type Boolean) (SweepResult :type Hit%20Result%20Structure%20%28by%20ref%29))
  (if (!= OtherActor self)
    (Game|Damage|ApplyDamage OtherActor (Math|Random|RandomFloatinRange 12.0 24.0) 0 0)))

(event OnComponentBeginOverlap(CapsuleLeftHand)
  (params (OverlappedComponent :type Primitive%20Component%20Object%20Reference) (OtherActor :type Actor%20Object%20Reference) (OtherComp :type Primitive%20Component%20Object%20Reference) (OtherBodyIndex :type Integer) (bFromSweep :type Boolean) (SweepResult :type Hit%20Result%20Structure%20%28by%20ref%29))
  (if (!= OtherActor self)
    (Game|Damage|ApplyDamage OtherActor (Math|Random|RandomFloatinRange 12.0 24.0) 0 0)))

(event Custom|Attack
  (if (not (Variables|Default|GetIsDeadMob?))
    (Utilities|FlowControl|DoOnce false
      (:Completed
        (Variables|/Script/Engine.CharacterMovementComponent|SetMaxWalkSpeed (Variables|Character|GetCharacterMovement) 0.0)
        (if (Math|Random|RandomBoolwithWeight 0.5)
          (Animation|PlayAnimMontage "/Game/Mob_and_Enemy/Mutant_Druid/Animations/Mutant_Attack_Montage.Mutant_Attack_Montage" 1.0 "None")
          (else
            (Animation|PlayAnimMontage "/Game/Mob_and_Enemy/Mutant_Druid/Animations/Mutant_Swiping_Montage.Mutant_Swiping_Montage" 1.0 "None")))))))

(event Custom|AttackEnded
  (bind _charactermovement (Variables|Character|GetCharacterMovement))
  (Variables|/Script/Engine.CharacterMovementComponent|SetMaxWalkSpeed _charactermovement (Variables|Default|GetStart%20Max%20Speed))
  (Utilities|FlowControl|DoOnce false) ; enters at Reset
)

(event Custom|Enable%20Collision%20Right%20Hand
  (Collision|SetCollisionEnabled (Variables|Default|GetCapsule%20Rigjt%20Hand) "QueryOnly"))

(event Custom|DisebleCollision%20Left%20Hand
  (Collision|SetCollisionEnabled (Variables|Default|GetCapsule%20Left%20Hand) "NoCollision"))

(event Custom|DisebleCollision%20Right%20Hand
  (Collision|SetCollisionEnabled (Variables|Default|GetCapsule%20Rigjt%20Hand) "NoCollision"))

(event Custom|Enable%20Collision%20Left%20Hand
  (Collision|SetCollisionEnabled (Variables|Default|GetCapsule%20Left%20Hand) "QueryOnly"))

(event Custom|Death
  (Variables|Default|SetIsDeadMob? true)
  (Default|Death (.AsBP%20Mutant%20Anim (Utilities|Casting|CastToBP_Mutant_Anim (Components|SkeletalMesh|GetAnimInstance (Variables|Character|GetMesh)))))
  (Animation|StopAnimMontage "/Game/Mob_and_Enemy/Mutant_Druid/Animations/Mutant_Attack_Montage.Mutant_Attack_Montage")
  (Animation|StopAnimMontage "/Game/Mob_and_Enemy/Mutant_Druid/Animations/Mutant_Swiping_Montage.Mutant_Swiping_Montage")
  (Collision|SetCollisionEnabled (Variables|Collision|GetCapsuleComponent) "NoCollision")
  (Utilities|FlowControl|Delay 1e+01)
  (Actor|DestroyActor))

(event EventBeginPlay
  (Variables|Default|SetRef%20HP%20Bar%20Widget (.AsHP%20Bar%20Widget (Utilities|Casting|CastToHP_Bar_Widget (UserInterface|GetUserWidgetObject (Variables|Default|GetHP_Bar)))))
  (Variables|Default|SetStart%20Max%20Speed (Variables|/Script/Engine.CharacterMovementComponent|GetMaxWalkSpeed (Variables|Character|GetCharacterMovement))))

(event Game|Damage|EventAnyDamage
  (params (Damage :type Float%20%28single-precision%29) (DamageType :type Damage%20Type%20Object%20Reference) (InstigatedBy :type Controller%20Object%20Reference) (DamageCauser :type Actor%20Object%20Reference))
  (if (not (Variables|Default|GetIsDeadMob?))
    (bind _output_get (Variables|Default|SetHP (Math|Float|SelectFloat 0.0 (- (Variables|Default|GetHP) Damage) (>= Damage (Variables|Default|GetHP)))))
    (if (<= _output_get 0.0)
      (CallFunction|Death))))

(event EventTick
  (params (DeltaSeconds :type Float%20%28single-precision%29))
  (bind _hp_bar (Variables|Default|GetHP_Bar))
  (bind _ref_hp_bar_widget (Variables|Default|GetRef%20HP%20Bar%20Widget))
  (Utilities|FlowControl|Sequence
    (:then_0
      (Progress|SetPercent (Variables|/Game/Mob_and_Enemy/Mutant_Druid/HP_Bar_Widget.HP_Bar_Widget_C|GetHP_Bar _ref_hp_bar_widget) (Math|Float|NormalizetoRange (Variables|Default|GetHP) 0.0 (Variables|Default|GetMax_HP)))
      (Rendering|Components|TextRender|SetText (Variables|/Game/Mob_and_Enemy/Mutant_Druid/HP_Bar_Widget.HP_Bar_Widget_C|GetMob_Name _ref_hp_bar_widget) (Variables|Default|GetMob_Name)))
    (:then_1
      ;[1 1 1] Сравнивает координаты и задает направление одного на другого
      (Transformation|SetWorldRotation _hp_bar (Math|Rotator|FindLookatRotation (Transformation|GetWorldLocation _hp_bar) (Transformation|GetWorldLocation (Variables|/Game/Mannequin/Archer/Blueprint/BP_Charapter.BP_Charapter_C|GetCameraTP (.AsBP%20Charapter (Utilities|Casting|CastToBP_Charapter (Game|GetPlayerCharacter 0)))))) false false))))

(fn ConstructionScript)