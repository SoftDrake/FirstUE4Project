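; Robot enemy character with a melee attack, health, death handling and an overhead health bar.
; Attack events play a DoOnce-gated montage and toggle a left-hand sphere that applies random damage on overlap.
; It registers in the player controller's target-lock list; at zero HP it plays a death animation, destroys itself after a delay and removes its entry.
; Tick refreshes the HP widget and rotates it toward the player's camera.
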(event OnComponentBeginOverlap(SphereLeftHand)
  (params (OverlappedComponent :type Primitive%20Component%20Object%20Reference) (OtherActor :type Actor%20Object%20Reference) (OtherComp :type Primitive%20Component%20Object%20Reference) (OtherBodyIndex :type Integer) (bFromSweep :type Boolean) (SweepResult :type Hit%20Result%20Structure%20%28by%20ref%29))
  (if (!= OtherActor self)
    (Game|Damage|ApplyDamage OtherActor (Math|Random|RandomFloatinRange 12.0 24.0) 0 0)))

(event Custom|RobotAttack
  (if (not (Variables|Default|GetIsDestroyRobot?))
    (Utilities|FlowControl|DoOnce false
      (:Completed
        (Animation|PlayAnimMontage "/Game/Mob_and_Enemy/Robot_Mob/Animation/Attack_Montage.Attack_Montage" 1.0 "None")))))

(event Custom|RobotAttackEnded
  (Utilities|FlowControl|DoOnce false) ; enters at Reset
)

(event Custom|Enable%20Collision%20Left%20Hand
  (Collision|SetCollisionEnabled (Variables|Default|GetSphereLeftHand) "QueryOnly"))

(event Custom|Desable%20Collision%20Left%20Hand
  (Collision|SetCollisionEnabled (Variables|Default|GetSphereLeftHand) "NoCollision"))

(event Custom|Death
  (bind _returnvalue (Game|GetPlayerController 0))
  (bind _asbp_player_controller (Utilities|Casting|CastToBP_PlayerController _returnvalue))
  (bind _ref_to_targetlock_actor (Variables|/Game/Mannequin/Archer/Blueprint/BP_PlayerController.BP_PlayerController_C|GetRef_To_TargetLock_Actor _asbp_player_controller))
  (Variables|Default|SetIsDestroyRobot? true)
  (Default|DeathAnim (.AsAnim%20BP%20Robot (Utilities|Casting|CastToAnimBP_Robot (Components|SkeletalMesh|GetAnimInstance (Variables|Character|GetMesh)))))
  (Animation|StopAnimMontage "/Game/Mob_and_Enemy/Robot_Mob/Animation/Attack_Montage.Attack_Montage")
  (Collision|SetCollisionEnabled (Variables|Collision|GetCapsuleComponent) "NoCollision")
  (Utilities|FlowControl|Delay 5.0)
  (Actor|DestroyActor)
  (for (_array_element _array_index) _ref_to_targetlock_actor
    (if (== _array_element self)
      (Utilities|Array|RemoveIndex _ref_to_targetlock_actor _array_index)
      (Utilities|Array|RemoveIndex (Variables|/Game/Mannequin/Archer/Blueprint/BP_PlayerController.BP_PlayerController_C|GetDistanceBetweenTarget _asbp_player_controller) _array_index))))

(event EventBeginPlay
  (bind _self self)
  (Variables|Default|SetRobotControllerSelf (Pawn|GetController))
  (Variables|Default|SetRobotSelf _self)
  (Utilities|Array|AddUnique (Variables|/Game/Mannequin/Archer/Blueprint/BP_PlayerController.BP_PlayerController_C|GetRef_To_TargetLock_Actor (.AsBP%20Player%20Controller (Utilities|Casting|CastToBP_PlayerController (Game|GetPlayerController 0)))) _self)
  (Variables|Default|SetHP_Bar_Robot_Ref (.AsHP%20Bar%20Robot%20Widget (Utilities|Casting|CastToHP_Bar_Robot_Widget (UserInterface|GetUserWidgetObject (Variables|Default|GetWidgetHP))))))

(event Game|Damage|EventAnyDamage
  (params (Damage :type Float%20%28single-precision%29) (DamageType :type Damage%20Type%20Object%20Reference) (InstigatedBy :type Controller%20Object%20Reference) (DamageCauser :type Actor%20Object%20Reference))
  (if (not (Variables|Default|GetIsDestroyRobot?))
    (bind _output_get (Variables|Default|SetCurrentHP (Math|Float|SelectFloat 0.0 (- (Variables|Default|GetCurrentHP) Damage) (>= Damage (Variables|Default|GetCurrentHP)))))
    (if (<= _output_get 0.0)
      (CallFunction|Death))))

(event EventTick
  (params (DeltaSeconds :type Float%20%28single-precision%29))
  (bind _hp_bar_robot_ref (Variables|Default|GetHP_Bar_Robot_Ref))
  (bind _widgethp (Variables|Default|GetWidgetHP))
  (Utilities|FlowControl|Sequence
    (:then_0
      (Progress|SetPercent (Variables|/Game/Mob_and_Enemy/Robot_Mob/BluePrint/HP_Bar_Robot_Widget.HP_Bar_Robot_Widget_C|GetHP_Bar_Robot _hp_bar_robot_ref) (Math|Float|NormalizetoRange (Variables|Default|GetCurrentHP) 0.0 (Variables|Default|GetMaxHP)))
      (Rendering|Components|TextRender|SetText (Variables|/Game/Mob_and_Enemy/Robot_Mob/BluePrint/HP_Bar_Robot_Widget.HP_Bar_Robot_Widget_C|GetRobot_Name _hp_bar_robot_ref) (Variables|Default|GetRobot_Name)))
    (:then_1
      (Transformation|SetWorldRotation _widgethp (Math|Rotator|FindLookatRotation (Transformation|GetWorldLocation _widgethp) (Transformation|GetWorldLocation (Variables|/Game/Mannequin/Archer/Blueprint/BP_Charapter.BP_Charapter_C|GetCameraTP (.AsBP%20Charapter (Utilities|Casting|CastToBP_Charapter (Game|GetPlayerCharacter 0)))))) false false))))

(event Collision|EventActorBeginOverlap
  (params (OtherActor :type Actor%20Object%20Reference)))

(fn ConstructionScript)