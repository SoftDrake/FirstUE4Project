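; Robot mob AI controller that runs an enemy behavior tree and feeds it perception results.
; Perception updates sort actors by "Enemy" tag or otherwise "Player", setting sight flags and target objects on the Blackboard.
; When sight fails, separate timers clear each target after a grace delay, longer for enemies than players, and a new sighting cancels the matching timer.
; Debug messages print on each sighting.
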(event OnTargetPerceptionUpdated(AIPerception)
  (params (Actor :type Actor%20Object%20Reference) (Stimulus :type AI%20Stimulus%20Structure))
  (bind _bsuccessfullysensed (Utilities|Struct|BreakAIStimulus Stimulus))
  (bind _output_get (Variables|Default|SetActorForTarget Actor))
  (if (Actor|ActorHasTag _output_get "Enemy")
    (AI|Components|Blackboard|SetValueasBool (Variables|Default|GetBlackboard) (Utilities|Name|MakeLiteralName "CanSeeEnemy") (and (Actor|ActorHasTag _output_get "Enemy") _bsuccessfullysensed))
    (if (and (Actor|ActorHasTag _output_get "Enemy") _bsuccessfullysensed)
      (Utilities|Time|ClearandInvalidateTimerbyHandle (Variables|Default|GetTimerEnemy))
      (AI|Components|Blackboard|SetValueasObject (Variables|Default|GetBlackboard) (Utilities|Name|MakeLiteralName "TargetEnemy") (Variables|Default|GetActorForTarget))
      (Development|PrintString "Вижу NPC")
      (else
        (bind _returnvalue (Utilities|Time|SetTimerbyEvent (delegate Custom|OnLostSightEnemy) 7.0))
        (Variables|Default|SetTimerEnemy _returnvalue)))
    (else
      (AI|Components|Blackboard|SetValueasBool (Variables|Default|GetBlackboard) (Utilities|Name|MakeLiteralName "CanSeePlayer") (and (Actor|ActorHasTag _output_get "Player") _bsuccessfullysensed))
      (if (and (Actor|ActorHasTag _output_get "Player") _bsuccessfullysensed)
        (Utilities|Time|ClearandInvalidateTimerbyHandle (Variables|Default|GetTimerPlayer))
        (AI|Components|Blackboard|SetValueasObject (Variables|Default|GetBlackboard) (Utilities|Name|MakeLiteralName "TargetActor") (Variables|Default|GetActorForTarget))
        (Development|PrintString "Вижу игрока")
        (else
          (bind _returnvalue_2 (Utilities|Time|SetTimerbyEvent (delegate Custom|OnLostSight) 3.0))
          (Variables|Default|SetTimerPlayer _returnvalue_2))))))

(event Custom|OnLostSight
  (AI|Components|Blackboard|SetValueasObject (Variables|Default|GetBlackboard) (Utilities|Name|MakeLiteralName "TargetActor") 0))

(event Custom|OnLostSightEnemy
  (AI|Components|Blackboard|SetValueasObject (Variables|Default|GetBlackboard) (Utilities|Name|MakeLiteralName "TargetEnemy") 0))

(event EventBeginPlay
  (AI|RunBehaviorTree "/Game/Mob_and_Enemy/Enemy_V_1/BehaviorTree_Task_Servise/Enemy_BehaviorTree.Enemy_BehaviorTree"))

(event EventTick
  (params (DeltaSeconds :type Float%20%28single-precision%29)))

(fn ConstructionScript)